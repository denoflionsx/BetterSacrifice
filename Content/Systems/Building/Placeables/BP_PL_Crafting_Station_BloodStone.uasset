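; Blood stone crafting station placeable where owners drag a thrall to convert it into an inventory item and show it sacrificed.
; Inventory changes drive visibility: the stored thrall's layout customizes the displayed body, chains, gender and voice, with clients waiting for replicated layout data.
; Animation events trigger blood sacrifice or soul drain, using timelines for channels, pool level and an emaciation material effect.
; Dedicated servers skip the visual setup.
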(event `self.ReceiveBeginPlay`
  ;[0 0.82 0.007598] Begin Play
  (`parent.ReceiveBeginPlay`)
  (if (`KismetSystemLibrary.IsDedicatedServer`)
    (`SkeletalMeshComponent.Stop` (`self.ThrallWorker`))
    (else
      (`|ExecutionSequence`
        (:`then_0`
          (`CharacterCustomizationComponent.SetMasterSkeletalMeshComponent` (`self.BP_CharacterCustomizationComponent`) (`self.ThrallWorker`) false)
          (if (`ItemInventory.IsInitialContentReceived` (`self.PlaceableInventory`))
            (if (`KismetSystemLibrary.IsServer`)
              (if (or (`PersistenceComponent.IsDataDoneLoading` (`self.PlaceableInventory`)) (not (`PersistenceComponent.m_bWasLoadedFromDB` (`self.PlaceableInventory`))))
                (`self.Handle Visibility`)
                (else
                  (add `PersistenceComponent.OnSignalDataLoaded` (`self.PlaceableInventory`) (`|CreateDelegate` :!event `Handle Visibility`))))
              (else
                (`self.Handle Visibility`)))
            (else
              (add `ItemInventory.SignalInventoryRecivedOnClient` (`self.PlaceableInventory`) (`|CreateDelegate` :!event `Handle Visibility`)))))
        (:`then_1`
          (if (not (`KismetSystemLibrary.IsServer`))
            (bind _returnvalue (`|GenericCreateObject` "/Script/ConanSandbox.ItemInventoryClientMonitor" self))
            (bind _output_get (set `self.InventoryMonitor` _returnvalue))
            (`ItemInventoryClientMonitor.SetInventory` _output_get (`self.PlaceableInventory`))))))))

(event `Handle Visibility`
  (bind _asab_human_sacrifice (cast `/Game/Master_AnimBP/AB_human_sacrifice` (`SkeletalMeshComponent.GetAnimInstance` (`self.ThrallWorker`)) :!pure true))
  ;[1 1 1] Handle Visibility (Thrall and Chains)
  (`|ExecutionSequence`
    (:`then_0`
      (bind _corpsedonoritem (`self.FindCorpseDonorItemFromStation`))
      (bind _output_get (set `self.CorpseDonorItem` _corpsedonoritem))
      (`/Engine/EditorBlueprintResources/StandardMacros.IsValid` _output_get
        (:`Is Valid`
          (if (not (`self.HasThrallItem`))
            (set `self.HasThrallItem` true)
            (`GameplayStatics.SpawnSoundAttached` "/Game/Sound/SFX/Sorcery/Rituals/Blood_Sacrifice/rit_blood_sacrifice_thrall_place_Cue.rit_blood_sacrifice_thrall_place_Cue" (`self.ThrallWorker`)))
          (`CharacterCustomizationComponent.SetEnabled` (`self.BP_CharacterCustomizationComponent`) true)
          (`self.DefineThrallAppearance`)
          (`self.ToggleChainVisibility` true)
          (`SkeletalMeshComponent.Play` (`self.ThrallWorker`) true)
          (`KismetSystemLibrary.Delay` 0.1) ; Make sure the animation has played for a bit.
          (`SceneComponent.SetVisibility` (`self.ThrallWorker`) true true))
        (:`Is Not Valid`
          (if (`self.HasThrallItem`)
            (set `self.HasThrallItem` false)
            (`SkeletalMeshComponent.Stop` (`self.ThrallWorker`))
            (`KismetSystemLibrary.Delay` 30.0)
            (if (not (`self.HasThrallItem`))
              (`CharacterCustomizationComponent.SetEnabled` (`self.BP_CharacterCustomizationComponent`) false :!label _label)
              (`self.ToggleChainVisibility` false)
              (`SceneComponent.SetVisibility` (`self.ThrallWorker`) false true)
              (`KismetSystemLibrary.Delay` 0.1) ; Wait a bit to make sure the animation stopping isn't viisble.
              (`SkeletalMeshComponent.Stop` (`self.ThrallWorker`))
              (`self.ResetShrinkAnim`)
              (set `/Game/Master_AnimBP/AB_human_sacrifice.drainsoul` false _asab_human_sacrifice)
              (set `/Game/Master_AnimBP/AB_human_sacrifice.bleedout` false _asab_human_sacrifice))
            (else
              (goto _label))))))
    (:`then_1`
      (`self.CheckBlood`))
    (:`then_2`
      (`self.SetVoice`))
    (:`then_3`
      (`self.SetGender`))))

(event `InteractableInterface.InteractableActivate`
  (params (Component :type "PrimitiveComponent Object Reference") (Instigator :type "PlayerController Object Reference") (HitIndex :type Integer) (TriggeredFromRadialWheel :type Boolean))
  (bind _returnvalue (`Controller.K2_GetPawn` Instigator))
  (bind _placeableinventory (`self.PlaceableInventory`))
  ;[1 1 1] Dragging a Thrall into the station
  (bind _returnvalue_2 (`ThrallOwnerInterface.IsDraggingThrall` (cast `ThrallOwnerInterface` _returnvalue :!pure true)))
  (if (and _returnvalue_2 (`self.IsOwner` _returnvalue))
    (if (and (== (`ItemInventory.FindItemByTemplateID` _placeableinventory 0 0) -1) (>= (`ItemInventory.GetFirstFreeIndex` _placeableinventory false) 0))
      (`ThrallOwnerInterface.StartThrallifyingPrisoner` (cast `ThrallOwnerInterface` _returnvalue :!pure true) self)
      (else
        (`ConanCharacter.ClientHUDShowNotification` (cast `ConanCharacter` _returnvalue :!pure true) "No more room on station" true)))
    (else
      (`parent.InteractableActivate` Component Instigator HitIndex TriggeredFromRadialWheel))))

(event `SetVoice`
  (bind _returnvalue (`KismetMathLibrary.RandomInteger` 8))
  ;[0.821 0.3001 1] Voice Set Assign
  (`/Engine/EditorBlueprintResources/StandardMacros.IsValid` (`self.CorpseDonorItem`)
    (:`Is Valid`
      (if (`self.IsThrallItemFemale`)
        (set `self.Voice` (`KismetArrayLibrary.Array_Get` (`self.FemaleVoices`) _returnvalue))
        (else
          (set `self.Voice` (`KismetArrayLibrary.Array_Get` (`self.MaleVoices`) _returnvalue)))))))

(event `CheckBlood`
  ;[1 1 1] Toggle Blood Pool Visibility
  (if (not (`KismetSystemLibrary.IsDedicatedServer`))
    (if (== (`ItemInventory.FindItemByTemplateID` (`self.PlaceableInventory`) 42000 0) -1)
      (if (`self.HasBlood`)
        (set `self.HasBlood` false)
        (`self.Blood Cleanup`))
      (else
        (set `self.HasBlood` true)
        (`SceneComponent.K2_SetWorldLocation` (`self.BloodPool`) (`SplineComponent.GetLocationAtSplinePoint` (`self.BloodSpline`) 1 "World") false false)))))

(event `OnThrallItemCharLayoutReceived`
  ;[1 1 1] Item is added/removed
  (bind _corpsedonoritem (`self.FindCorpseDonorItemFromStation` :!label _label_2))
  (`/Engine/EditorBlueprintResources/StandardMacros.IsValid` _corpsedonoritem
    (:`Is Valid`
      (`self.CheckThrallItemCharLayoutIsDefined` _corpsedonoritem
        (:`IsNotDefined`
          (add `ThrallItem.SignalReceivedCharacterLayout` _corpsedonoritem (delegate `OnThrallItemCharLayoutReceived`)))
        (:`IsDefined`
          (`self.Handle Visibility`))))))

(event `self.PlaceableInventory.SignalItemAdded`
  (params (index :type Integer) (item :type "GameItem Object Reference") (srcInventory :type "ItemInventory Object Reference") (srcIndex :type Integer))
  ;[1 1 1] Item is added/removed
  (if (not (`KismetSystemLibrary.IsDedicatedServer`))
    (`self.CheckBlood`)
    (if (not (`KismetSystemLibrary.IsServer`))
      (goto _label_2)
      (else
        (`self.Handle Visibility`)))))

(event `SetGender`
  (bind _asab_human_sacrifice (cast `/Game/Master_AnimBP/AB_human_sacrifice` (`SkeletalMeshComponent.GetAnimInstance` (`self.ThrallWorker`)) :!pure true))
  ;[1 1 1] Set gender for the animation
  (if (`self.IsThrallItemFemale`)
    (set `/Game/Master_AnimBP/AB_human_sacrifice.Isfemale` true _asab_human_sacrifice)
    (else
      (set `/Game/Master_AnimBP/AB_human_sacrifice.Isfemale` false _asab_human_sacrifice))))

(event `self.PlaceableInventory.SignalItemRemoved`
  (params (index :type Integer) (item :type "GameItem Object Reference") (dstInventory :type "ItemInventory Object Reference") (dstIndex :type Integer))
  ;[1 1 1] Item is added/removed
  (if (not (`KismetSystemLibrary.IsDedicatedServer`))
    (`/Engine/EditorBlueprintResources/StandardMacros.IsValid` (`self.ActiveRitual`)
      (:`Is Valid`
        (`self.CheckBlood`))
      (:`Is Not Valid`
        (bind _corpsedonoritem (`self.FindCorpseDonorItemFromStation`))
        (`/Engine/EditorBlueprintResources/StandardMacros.IsValid` _corpsedonoritem
          (:`Is Not Valid`
            (set `self.HasThrallItem` false)))))
    (`self.Handle Visibility`)))

(event `/Game/Systems/Thrall/ThrallConverterInterface.ConverThrall`
  (params (ThrallActor :type "Actor Object Reference"))
  ;[1 1 1] Create the ThrallItem
  (bind _asconan_character (cast `ConanCharacter` ThrallActor))
  (bind _layout (message `HasCharacterLayoutInterface.GetCharacterLayout` _asconan_character))
  (bind _returnvalue (`GameItemSpawner.SpawnThrallItem` "/Script/ConanSandbox.ThrallItem" _asconan_character _layout))
  (bind _returnvalue_2 (`GameMetricsLibrary.GetItemOperationCraftingContext` self))
  (`ItemInventory.AddItem` (`self.PlaceableInventory`) _returnvalue _returnvalue_2 -1)
  (`ConanCharacter.ConvertedToThrall` _asconan_character))

(event `TimeToDie`
  (bind (_asab_human_sacrifice _bsuccess) (cast `/Game/Master_AnimBP/AB_human_sacrifice` (`SkeletalMeshComponent.GetAnimInstance` (`self.ThrallWorker`)) :!pure true))
  ;[0.3039 0 1] Blood Sacrifice - Thrall
  (if _bsuccess
    (set `/Game/Master_AnimBP/AB_human_sacrifice.bleedout` true _asab_human_sacrifice)))

(event `TimeToDrain`
  (bind (_asab_human_sacrifice _bsuccess) (cast `/Game/Master_AnimBP/AB_human_sacrifice` (`SkeletalMeshComponent.GetAnimInstance` (`self.ThrallWorker`)) :!pure true))
  ;[0.01928 0.7995 1] Soul Sacrifice - Thrall
  (if _bsuccess
    (set `self.SacrificeAnimBP` _asab_human_sacrifice)
    (`|ExecutionSequence`
      (:`then_0`
        (`KismetArrayLibrary.Array_Clear` (`self.ThrallMatInstances`))
        (for _array_element (`self.K2_GetComponentsByClass` "/Script/Engine.SkeletalMeshComponent")
          (for _array_element_2 (`MeshComponent.GetMaterials` _array_element)
            (bind _asmaterial_instance_dynamic (cast `MaterialInstanceDynamic` _array_element_2))
            (`KismetArrayLibrary.Array_Add` (`self.ThrallMatInstances`) _asmaterial_instance_dynamic)))
        (`self.PlayShrinkAnim`))
      (:`then_1`
        (set `/Game/Master_AnimBP/AB_human_sacrifice.drainsoul` true _asab_human_sacrifice)
        (`KismetSystemLibrary.Delay` 7.0)
        (`ActorComponent.Activate` (`self.Particles_DrainSoul`) true)
        (`GameplayStatics.SpawnSoundAtLocation` "/Game/Sound/SFX/Sorcery/Rituals/Soul_Drain/rit_soul_drain_cast_Cue.rit_soul_drain_cast_Cue" (`SceneComponent.K2_GetComponentLocation` (`self.Particles_DrainSoul`)))
        (`GameplayStatics.SpawnSoundAtLocation` "/Game/Sound/SFX/Sorcery/Rituals/Soul_Drain/rit_soul_drain_skin_shrink_Cue.rit_soul_drain_skin_shrink_Cue" (`SceneComponent.K2_GetComponentLocation` (`self.ThrallWorker`)))))))

(event `SlitThroat`
  (bind _bloodripple (`self.BloodRipple`))
  ;[0.3039 0 1] Blood Sacrifice - Station
  (`SceneComponent.SetVisibility` _bloodripple true true)
  (`SceneComponent.SetVisibility` (`self.BloodChannels`) true true)
  (`SceneComponent.SetHiddenInGame` _bloodripple false true)
  (`SceneComponent.SetHiddenInGame` (`self.BloodChannels`) false true)
  (bind (_direction _blood_level _bloodchannels _ripple_size) (`Timeline|Timeline_0` :!label _label)
    (:`Update`
      (`MeshComponent.SetScalarParameterValueOnMaterials` (`self.BloodChannels`) "Blood Level" _bloodchannels)
      (`SceneComponent.SetRelativeScale3D` (`self.BloodRipple`) _ripple_size)
      (`SceneComponent.K2_SetWorldLocation` (`self.BloodPool`) (`KismetMathLibrary.VLerp` (`SplineComponent.GetLocationAtSplinePoint` (`self.BloodSpline`) 0 "World") (`SplineComponent.GetLocationAtSplinePoint` (`self.BloodSpline`) 1 "World") _blood_level) false false))))

(event `Blood Cleanup`
  ;[0.3039 0 1] Blood Sacrifice - Station
  (`SceneComponent.SetVisibility` (`self.BloodRipple`) false true)
  (`SceneComponent.SetVisibility` (`self.BloodChannels`) false true)
  (goto _label :!via `ReverseFromEnd`))

(event `PlayShrinkAnim`
  (bind _sacrificeanimbp (`self.SacrificeAnimBP`))
  ;[0.01928 0.7995 1] Soul Sacrifice - Shrinking Material Anim
  (bind (_direction _shrink _corrupt _normal) (`Timeline|Emaciate_Timeline` :!label _label_2)
    (:`Update`
      (`/Engine/EditorBlueprintResources/StandardMacros.IsValid` _sacrificeanimbp
        (:`Is Valid`
          (set `/Game/Master_AnimBP/AB_human_sacrifice.Shrink` _shrink _sacrificeanimbp))
        (:`Is Not Valid`
          _))
      (for _array_element (`self.ThrallMatInstances`)
        (`MaterialInstanceDynamic.SetScalarParameterValue` _array_element "corruption" _corrupt)
        (`MaterialInstanceDynamic.SetScalarParameterValue` _array_element "NormalStrength" _normal)
        (`MaterialInstanceDynamic.SetVectorParameterValue` _array_element "CorruptedVeinTint" (struct :`R` 1.0 :`G` 1.0 :`B` 1.0 :`A` 1.0))
        (`MaterialInstanceDynamic.SetVectorParameterValue` _array_element "CorruptedSkinTint" (struct :`R` 0.19 :`G` 0.189191 :`B` 0.159789 :`A` 1.0))
        (`MaterialInstanceDynamic.SetVectorParameterValue` _array_element "CorruptedSkinTintSS" (struct :`A` 1.0))
        (`MaterialInstanceDynamic.SetVectorParameterValue` _array_element "FresnelTintCorrupted" (struct :`R` 1.0 :`G` 1.0 :`B` 1.0 :`A` 1.0))))))

(event `ResetShrinkAnim`
  ;[0.01928 0.7995 1] Soul Sacrifice - Shrinking Material Anim
  (goto _label_2 :!via `SetNewTime`))

(fn `FindCorpseDonorItemFromStation`
  (returns (CorpseDonorItem :type "ThrallItem Object Reference"))
  (for _array_element (`ItemInventory.ItemList` (`self.PlaceableInventory`))
    (`/Engine/EditorBlueprintResources/StandardMacros.IsValid` _array_element
      (:`Is Valid`
        (bind _asthrall_item (cast `ThrallItem` _array_element))
        (return _asthrall_item))))
  (return null))

(fn `ToggleChainVisibility`
  (params (ThrallPresent :type Boolean))
  (bind _chains_skinned (`self.Chains_Skinned`))
  (if ThrallPresent
    (`SceneComponent.SetVisibility` (`self.Chains_Neutral`) false true)
    (`SceneComponent.SetVisibility` (`self.Chains_Active`) true true)
    (`SkinnedMeshComponent.SetSkinnedAssetAndUpdate` _chains_skinned (select `bool` (`self.IsThrallItemFemale`) :`false` "/Game/Environment/Player_built/Meshes/SK_bloodritual_sacrificialstone_chains_male.SK_bloodritual_sacrificialstone_chains_male" :`true` "/Game/Environment/Player_built/Meshes/SK_bloodritual_sacrificialstone_chains_female.SK_bloodritual_sacrificialstone_chains_female" :!type "SkeletalMesh Object Reference") true)
    (`SkinnedMeshComponent.SetLeaderPoseComponent` _chains_skinned (`self.ThrallWorker`))
    (`SceneComponent.SetVisibility` _chains_skinned true false)
    (else
      (`SceneComponent.SetVisibility` (`self.Chains_Neutral`) true true)
      (`SceneComponent.SetVisibility` (`self.Chains_Active`) false true)
      (`SceneComponent.SetVisibility` (`self.Chains_Skinned`) false false))))

(fn `UserConstructionScript`)